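; Enemy Blueprint that chases the player and can be killed by damage.
; BeginPlay enters a FlipFlop whose first output starts TargetPlayer, a delayed self-repeating AIMoveTo loop; the second leads to RandomRoam, which moves to a random reachable point before chasing.
; TargetAnimal is a similar loop with no target set and no outside caller here.
; AnyDamage reduces Health, then at zero destroys the actor and calls OnEliminated.
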(event `self.ReceiveBeginPlay`
  (`/Engine/EditorBlueprintResources/StandardMacros.FlipFlop`
    (:`A`
      (`self.TargetPlayer`))
    (:`B`
      (`self.RandomRoam`))))

(event `RandomRoam`
  ;[0.824 0.2438 0.1035 0.5] Enemy Movement
  (`|AIMoveTo` self (`NavigationSystemV1.K2_GetRandomReachablePointInRadius` (`self.K2_GetActorLocation`) 2000.0 null null) null 50.0
    (:`OnSuccess`
      (`KismetSystemLibrary.Delay` (`KismetMathLibrary.RandomFloatInRange` 1.0 2.0))
      (`self.TargetPlayer`))))

(event `TargetPlayer`
  ;[0.824 0.2438 0.1035 0.5] Enemy Movement
  (`|AIMoveTo` self (0.0 0.0 0.0) (`GameplayStatics.GetPlayerCharacter` 0) 50.0
    (:`then`
      (`KismetSystemLibrary.PrintString` "Chasing player" true true (struct :`G` 0.66 :`B` 1.0 :`A` 1.0) 4.0))
    (:`OnSuccess`
      (`KismetSystemLibrary.Delay` (`KismetMathLibrary.RandomFloatInRange` 1.0 2.0))
      (`self.TargetPlayer`))))

(event `TargetAnimal`
  ;[0.824 0.2438 0.1035 0.5] Enemy Movement
  (`|AIMoveTo` self (0.0 0.0 0.0) null
    (:`then`
      (`KismetSystemLibrary.PrintString` "Chasing Animal" true true (struct :`G` 0.66 :`B` 1.0 :`A` 1.0) 8.0))
    (:`OnSuccess`
      (`KismetSystemLibrary.Delay` (`KismetMathLibrary.RandomFloatInRange` 1.0 2.0))
      (`self.TargetAnimal`))))

(event `self.ReceiveAnyDamage`
  (params (Damage :type "Float (single-precision)") (DamageType :type "DamageType Object Reference") (InstigatedBy :type "Controller Object Reference") (DamageCauser :type "Actor Object Reference"))
  ;[0.07283 0.449 0 0.5] Health
  (set `self.Health` (- (`self.Health`) Damage))
  (if (<= (`self.Health`) 0.0)
    (`KismetSystemLibrary.PrintString` "Enemy is Dead!")
    (`self.K2_DestroyActor`)
    (`self.OnEliminated`)
    (else
      (`KismetSystemLibrary.PrintString` (`KismetStringLibrary.Concat_StrStr` "Enemy has " (`KismetStringLibrary.Conv_DoubleToString` (`self.Health`)) " HP left")))))

(fn `UserConstructionScript`)