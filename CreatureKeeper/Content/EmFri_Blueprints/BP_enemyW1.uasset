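; BP_enemyW1 is a bat enemy that supplies hurt, death and attack behaviour through events.
; Hurt and death play one-shot animations, and death waits briefly before notifying the Manager and destroying the actor.
; Attack plays its animation and immediately damages the player if within DamageRange, then calls TargetPlayer, after a delay on a hit or at once on a miss.
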(event `self.GetHurt`
  (`SkeletalMeshComponent.PlayAnimation` (`self.Mesh`) "/Game/Assets/FBX/Bat_Anim_BatArmature_Bat_Hit.Bat_Anim_BatArmature_Bat_Hit" false))

(event `self.Die`
  (`SkeletalMeshComponent.PlayAnimation` (`self.Mesh`) "/Game/Assets/FBX/Bat_Anim_BatArmature_Bat_Death.Bat_Anim_BatArmature_Bat_Death" false)
  (`KismetSystemLibrary.Delay` 2.0)
  (`/Game/BluePrints/EnemieWaveStuff/BP_EnemySpawnManager.RemoveEnemyAndCheck` (`self.Manager`))
  (`self.K2_DestroyActor`))

(event `self.Attack`
  (`SkeletalMeshComponent.PlayAnimation` (`self.Mesh`) "/Game/Assets/FBX/Bat_Anim_BatArmature_Bat_Attack.Bat_Anim_BatArmature_Bat_Attack" false)
  (if (<= (`KismetMathLibrary.Vector_Distance` (`SceneComponent.K2_GetComponentLocation` (`self.Mesh`)) (`CharacterMovementComponent.GetLastUpdateLocation` (`Character.CharacterMovement` (`GameplayStatics.GetPlayerCharacter` 0)))) (`self.DamageRange`))
    (`GameplayStatics.ApplyDamage` (`GameplayStatics.GetPlayerCharacter` 0) (`self.Damage`))
    (`KismetSystemLibrary.PrintString` "Enemy Attacked Player")
    (`KismetSystemLibrary.Delay` 5.0)
    (else
      (`KismetSystemLibrary.PrintString` "Enemy Attack Missed!")))
  (`self.TargetPlayer`))

(fn `UserConstructionScript`
  (`parent.UserConstructionScript`))