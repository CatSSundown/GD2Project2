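; BP_Animal is a roaming animal that takes damage and can be killed.
; From BeginPlay it loops AI MoveTo toward random reachable points around itself, pausing briefly after each success; a failed move ends the loop.
; AnyDamage reduces Health and prints what remains.
; At zero or below it prints a death message, destroys the actor, then calls the OnEliminated dispatcher.
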(event `self.ReceiveBeginPlay`
  (`self.RandomRoam`))

(event `RandomRoam`
  (`|AIMoveTo` self (`NavigationSystemV1.K2_GetRandomReachablePointInRadius` (`self.K2_GetActorLocation`) 2000.0 null null) null 10.0
    (:`OnSuccess`
      (`KismetSystemLibrary.Delay` (`KismetMathLibrary.RandomFloatInRange` 1.0 2.0))
      (`self.RandomRoam`))))

(event `self.ReceiveAnyDamage`
  (params (Damage :type "Float (single-precision)") (DamageType :type "DamageType Object Reference") (InstigatedBy :type "Controller Object Reference") (DamageCauser :type "Actor Object Reference"))
  ;[0.1693 0.5823 0.06978 0.5] Health
  (set `self.Health` (- (`self.Health`) Damage))
  (if (<= (`self.Health`) 0.0)
    (`KismetSystemLibrary.PrintString` "Animal is Dead!")
    (`self.K2_DestroyActor`)
    (`self.OnEliminated`)
    (else
      (`KismetSystemLibrary.PrintString` (`KismetStringLibrary.Concat_StrStr` "Animal has " (`KismetStringLibrary.Conv_DoubleToString` (`self.Health`)) " HP left")))))

(fn `UserConstructionScript`)