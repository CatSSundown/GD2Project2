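; BP_Base is an actor with a Health value whose destruction loses the game.
; Incoming damage is subtracted from Health in the AnyDamage event, and the remaining value is printed while it stays above zero.
; When Health runs out, it shows the W_LoseScreen widget, waits briefly, then quits the game.
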(event `self.ReceiveAnyDamage`
  (params (Damage :type "Float (single-precision)") (DamageType :type "DamageType Object Reference") (InstigatedBy :type "Controller Object Reference") (DamageCauser :type "Actor Object Reference"))
  (set `self.Health` (- (`self.Health`) Damage))
  (if (<= (`self.Health`) 0.0)
    (`KismetSystemLibrary.PrintString` "Death")
    (bind _returnvalue (`|CreateWidget` "/Game/Widgets/W_LoseScreen.W_LoseScreen_C"))
    (`UserWidget.AddToViewport` _returnvalue 0)
    (`KismetSystemLibrary.Delay` 2.0)
    (`KismetSystemLibrary.QuitGame` null "Quit")
    (else
      (`KismetSystemLibrary.PrintString` (`KismetStringLibrary.Conv_DoubleToString` (`self.Health`))))))

(fn `UserConstructionScript`)