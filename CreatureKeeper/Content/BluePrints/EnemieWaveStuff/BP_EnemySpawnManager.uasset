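; Enemy wave manager that runs three waves and ends the game with a win screen when all are cleared.
; After a delay on BeginPlay it gathers three spawner classes; WavesPassed counts down to pick the wave, each spawning its enemy type at spawner transforms, wave two adding first-wave enemies.
; Spawned enemies get a manager reference; RemoveEnemyAndCheck tracks the total, showing a wave banner before the next wave.
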(event `self.ReceiveBeginPlay`
  ; Get All Spawners and spawn first wave
  (`KismetSystemLibrary.Delay` 5.0)
  (`KismetSystemLibrary.PrintString` "Enemy Spawn Manager is Ready")
  (bind _outactors (`GameplayStatics.GetAllActorsOfClass` "/Game/BluePrints/EnemieWaveStuff/BP_TestEnemySpawner.BP_TestEnemySpawner_C"))
  (set `self.Out Actors` _outactors)
  (bind _outactors_2 (`GameplayStatics.GetAllActorsOfClass` "/Game/BluePrints/EnemieWaveStuff/BP_TestEnemySpawner2.BP_TestEnemySpawner2_C"))
  (set `self.Out Actors_2` _outactors_2)
  (bind _outactors_3 (`GameplayStatics.GetAllActorsOfClass` "/Game/BluePrints/EnemieWaveStuff/BP_TestEnemySpawner3.BP_TestEnemySpawner3_C"))
  (set `self.Out Actors_3` _outactors_3)
  (`self.EnemyWaveCheck`))

(event `EnemyWaveCheck`
  ;[0.02248 0.03272 0.15 0.5] Checks What wave it is
  (if (== (`self.WavesPassed`) 3)
    (`self.Spawn Enemies`)))

(event `EnemyWaveCheck2`
  ;[0.02248 0.03272 0.15 0.5] Checks What wave it is
  (if (== (`self.WavesPassed`) 2)
    (`self.SpawnWave2`)))

(event `EnemyWaveCheck3`
  ;[0.02248 0.03272 0.15 0.5] Checks What wave it is
  (if (== (`self.WavesPassed`) 1)
    (`self.SpawnWave3`)))

(event `Spawn Enemies`
  ;[0.15 0.002031 0.002031 0.5] Spawn Enemys each wave
  (for _array_element (`self.Out Actors`)
    (`/Engine/EditorBlueprintResources/StandardMacros.Do N` 30
      (:`Exit`
        (bind (_returnvalue_location _returnvalue_rotation) (`KismetMathLibrary.BreakTransform` (`SceneComponent.K2_GetComponentToWorld` (`Actor.RootComponent` _array_element))))
        (bind _returnvalue (`|SpawnActorFromClass` "/Game/EmFri_Blueprints/BP_enemyW1.BP_enemyW1_C" (`KismetMathLibrary.MakeTransform` _returnvalue_location _returnvalue_rotation) "Undefined" "MultiplyWithRoot" null null)) ; Create a new enemy at the spawner's location and rotation.
        (set `/Game/EmFri_Blueprints/BP_enemyW1.Manager` self _returnvalue)
        (`/Engine/EditorBlueprintResources/StandardMacros.IncrementInt` (`self.CurrentEnemyTotal`))))))

(event `SpawnWave2`
  ;[0.15 0.002031 0.002031 0.5] Spawn Enemys each wave
  (`/Engine/EditorBlueprintResources/StandardMacros.Do N` 30
    (:`Exit`
      (for _array_element (`self.Out Actors_2`)
        (bind (_returnvalue_location _returnvalue_rotation) (`KismetMathLibrary.BreakTransform` (`SceneComponent.K2_GetComponentToWorld` (`Actor.RootComponent` _array_element))))
        (bind _returnvalue (`|SpawnActorFromClass` "/Game/EmFri_Blueprints/BP_enemyW2.BP_enemyW2_C" (`KismetMathLibrary.MakeTransform` _returnvalue_location _returnvalue_rotation) "Undefined" "MultiplyWithRoot" null null)) ; Create a new enemy at the spawner's location and rotation.
        (set `/Game/EmFri_Blueprints/BP_enemyW2.Manager2` self _returnvalue)
        (`/Engine/EditorBlueprintResources/StandardMacros.IncrementInt` (`self.CurrentEnemyTotal`)
          (:`  `
            (for _array_element_2 (`self.Out Actors`)
              (`/Engine/EditorBlueprintResources/StandardMacros.Do N` 3
                (:`Exit`
                  (bind (_returnvalue_location_2 _returnvalue_rotation_2) (`KismetMathLibrary.BreakTransform` (`SceneComponent.K2_GetComponentToWorld` (`Actor.RootComponent` _array_element_2))))
                  (bind _returnvalue_2 (`|SpawnActorFromClass` "/Game/EmFri_Blueprints/BP_enemyW1.BP_enemyW1_C" (`KismetMathLibrary.MakeTransform` _returnvalue_location_2 _returnvalue_rotation_2) "Undefined" "MultiplyWithRoot" null null)) ; Create a new enemy at the spawner's location and rotation.
                  (set `/Game/EmFri_Blueprints/BP_enemyW1.Manager` self _returnvalue_2)
                  (`/Engine/EditorBlueprintResources/StandardMacros.IncrementInt` (`self.CurrentEnemyTotal`)))))))))))

(event `SpawnWave3`
  ;[0.15 0.002031 0.002031 0.5] Spawn Enemys each wave
  (`/Engine/EditorBlueprintResources/StandardMacros.Do N` 30
    (:`Exit`
      (for _array_element (`self.Out Actors_3`)
        (bind (_returnvalue_location _returnvalue_rotation) (`KismetMathLibrary.BreakTransform` (`SceneComponent.K2_GetComponentToWorld` (`Actor.RootComponent` _array_element))))
        (bind _returnvalue (`|SpawnActorFromClass` "/Game/EmFri_Blueprints/BP_enemyW3.BP_enemyW3_C" (`KismetMathLibrary.MakeTransform` _returnvalue_location _returnvalue_rotation) "Undefined" "MultiplyWithRoot" null null)) ; Create a new enemy at the spawner's location and rotation.
        (set `/Game/EmFri_Blueprints/BP_enemyW3.Manager3` self _returnvalue)
        (`/Engine/EditorBlueprintResources/StandardMacros.IncrementInt` (`self.CurrentEnemyTotal`))))))

(event `RemoveEnemyAndCheck`
  ;[0 2.4e-05 0.15 0.5] Removes Enemies and Checks for when all waves are over
  (`/Engine/EditorBlueprintResources/StandardMacros.DecrementInt` (`self.CurrentEnemyTotal`)
    (:`  `
      (if (not (> (`self.CurrentEnemyTotal`) 0))
        (`/Engine/EditorBlueprintResources/StandardMacros.DecrementInt` (`self.WavesPassed`)
          (:`  `
            (if (== (`self.WavesPassed`) 0)
              (`self.WaveCheck`)
              (else
                (`KismetSystemLibrary.PrintString` "NEW WAVE INCOMING" true true (struct :`G` 0.66 :`B` 1.0 :`A` 1.0) 5.0)
                (bind _returnvalue (`|CreateWidget` "/Game/Widgets/W_WaveText.W_WaveText_C"))
                (`UserWidget.AddToViewport` _returnvalue 0)
                (`KismetSystemLibrary.Delay` 5.0)
                (`Widget.RemoveFromParent` _returnvalue)
                (if true
                  (if (== (`self.WavesPassed`) 2)
                    (`self.EnemyWaveCheck2`)
                    (elif (== (`self.WavesPassed`) 1)
                      (`self.EnemyWaveCheck3`))))))))))))

(event `WaveCheck`
  ;[0.0252 0.15 0.04456 0.5] Ends The Game
  (if (== (`self.WavesPassed`) 0)
    (`KismetSystemLibrary.PrintString` "All Waves Cleared!")
    (bind _returnvalue (`|CreateWidget` "/Game/Widgets/W_Winscreen.W_Winscreen_C"))
    (`UserWidget.AddToViewport` _returnvalue 0)
    (`KismetSystemLibrary.Delay` 2.0)
    (`KismetSystemLibrary.QuitGame` null "Quit")))

(fn `UserConstructionScript`)